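; Paint ball projectile that leaves a decal actor, aligned to the surface normal, where it hits anything but the ThirdPersonCharacter, then destroys itself.
; The construction script sets velocity from Velo with a slight upward offset, shrinks the ball and starts a fast looping timer.
; That timer cycles the point light and material color through time-based sine waves, calling CreateDynamicMaterialInstance on every tick.
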(event OnComponentHit(paint)
  (params (HitComponent :type Primitive%20Component%20Object%20Reference) (OtherActor :type Actor%20Object%20Reference) (OtherComp :type Primitive%20Component%20Object%20Reference) (NormalImpulse :type Vector :default "0, 0, 0") (Hit :type Hit%20Result%20Structure%20%28by%20ref%29))
  (bind (_bblockinghit _binitialoverlap _time _distance _location _impactpoint _normal _impactnormal) (Collision|BreakHitResult Hit))
  ;[1 1 1] Anything BUT the player
  (Utilities|Casting|CastToThirdPersonCharacter OtherActor
    (:CastFailed
      ;[1 1 1] Instantiate decal and destroy the ball
      (Game|SpawnActorfromClass "/Game/DecalActor_Blueprint.DecalActor_Blueprint_C" (Math|Transform|MakeTransform _impactpoint (Math|Conversions|RotationFromXVector _impactnormal) "1,1,1") "Undefined" 0 0)
      (Actor|DestroyActor))))

(fn ConstructionScript
  ;[1 1 1] Set ball's direction
  (Variables|/Script/Engine.MovementComponent|SetVelocity (Variables|Default|GetProjectileMovement) (+ (Variables|Default|Getvelo) "0, 0,0.600000"))
  (Transformation|SetActorScale3D "0.250000,0.250000,0.250000")
  (CallFunction|Changecolor))

(fn Changecolor
  (Utilities|Time|SetTimerbyFunctionName 0 "loop" 0.01 true))

(fn Loop
  (bind _returnvalue (Actor|GetGameTimeSinceCreation))
  (bind _returnvalue_2 (* _returnvalue 3.5e+02))
  (bind _returnvalue_3 (* _returnvalue 3e+02))
  (bind _returnvalue_4 (* _returnvalue 4e+02))
  (bind _returnvalue_5 (Math|Trig|Sin(Degrees) _returnvalue_2))
  (bind _returnvalue_6 (Math|Trig|Sin(Degrees) _returnvalue_3))
  (bind _returnvalue_7 (Math|Trig|Sin(Degrees) _returnvalue_4))
  (bind _returnvalue_8 (Math|Float|Absolute(Float) _returnvalue_7))
  (bind _returnvalue_9 (Math|Float|Absolute(Float) _returnvalue_6))
  (bind _returnvalue_10 (Math|Float|Absolute(Float) _returnvalue_5))
  (Rendering|Components|Light|SetLightColor (Variables|Default|GetPointLight) (Utilities|Struct|MakeLinearColor _returnvalue_9 _returnvalue_10 _returnvalue_8 1.0) true)
  (bind _returnvalue_11 (Rendering|Material|CreateDynamicMaterialInstance (Variables|Default|Getpaint) 0 0 "None" :!class /Script/Engine.PrimitiveComponent))
  (Rendering|Material|SetVectorParameterValue _returnvalue_11 "param" (Utilities|Struct|MakeLinearColor _returnvalue_9 _returnvalue_10 _returnvalue_8 1.0) :!class /Script/Engine.MaterialInstanceDynamic))